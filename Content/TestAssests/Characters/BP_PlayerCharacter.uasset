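; Player character Blueprint that relays melee combo and hit moments to the Gameplay Ability System as gameplay events.
; Combo start, continue and reset events send matching Attack tags to the character itself.
; AttackHandle sphere-overlaps at the left hand socket and sends Attack.Hit with target data to the first AI character found.
; An older counter-based montage combo remains in the graph, disconnected and never run.
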(event Custom|ComboContimue
  (Ability|SendGameplayEventtoActor self "(TagName=\"Attack.ComboContinue\")"))

(event Custom|Attack%20Handle
  (bind _outactors (Collision|SphereOverlapActors (Transformation|GetSocketLocation (Variables|Character|GetMesh) "hand_l") 5e+01 (Utilities|Array|MakeArray "ObjectTypeQuery3") "/Game/TestAssests/Characters/BP_AICharacter.BP_AICharacter_C" (Utilities|Array|MakeArray self)))
  (if (Utilities|Array|IsValidIndex _outactors)
    (Ability|SendGameplayEventtoActor (Utilities|Array|Get(acopy) _outactors) "(TagName=\"Attack.Hit\")" (Utilities|Struct|MakeGameplayEventData "(TagName=\"\")" (Game|GetInstigator) (Utilities|Array|Get(acopy) _outactors) 0 0 "()" "(GameplayTags=)" "(GameplayTags=)" 0.0 (Ability|TargetData|AbilityTargetDatafromActor (Utilities|Array|Get(acopy) _outactors))))))

(event Custom|ComboStart
  (Ability|SendGameplayEventtoActor self "(TagName=\"Attack.ComboStart\")"))

(event Custom|ComboReset
  (Ability|SendGameplayEventtoActor self "(TagName=\"Attack.ComboReset\")"))

(fn ConstructionScript)