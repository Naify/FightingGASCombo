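; Gameplay Ability for a three-stage melee combo that plays elbow, jab and quad montages at increased speed.
; Gameplay events open each follow-up window, where an input press plays the next montage, while Attack.ComboReset ends the ability.
; It also ends when the jab is interrupted or the final montage completes, blends out or is interrupted.
; Hit handling that would fire a GameplayCue and forward Attack.Hit to the target is unconnected and never runs.
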(event Ability|EventActivateAbility
  (Animation|Montage|PlayMontage (.skeletalmeshcomponent (Ability|GetActorInfo)) "/Game/TestAssests/Animations/Player/Combat/AM_Elbow.AM_Elbow" 1.5
    (:then
      (Ability|Tasks|WaitGameplayEvent "(TagName=\"Attack.ComboStart\")" 0 true
        (:then
          (Ability|Tasks|WaitGameplayEvent "(TagName=\"Attack.ComboReset\")" 0 true
            (:EventReceived
              (Ability|EndAbility))))
        (:EventReceived
          (Ability|Tasks|WaitInputPress false
            (:OnPress
              (Animation|Montage|PlayMontage (.skeletalmeshcomponent (Ability|GetActorInfo)) "/Game/TestAssests/Animations/Player/Combat/AM_Jab.AM_Jab" 1.5
                (:then
                  (Ability|Tasks|WaitGameplayEvent "(TagName=\"Attack.ComboContinue\")" 0 true
                    (:then
                      (Ability|Tasks|WaitGameplayEvent "(TagName=\"Attack.ComboReset\")" 0 true
                        (:EventReceived
                          (Ability|EndAbility))))
                    (:EventReceived
                      (Ability|Tasks|WaitInputPress false
                        (:OnPress
                          (Animation|Montage|PlayMontage (.skeletalmeshcomponent (Ability|GetActorInfo)) "/Game/TestAssests/Animations/Player/Combat/AM_Quad.AM_Quad" 1.5
                            (:OnCompleted
                              _)
                            (:OnBlendOut
                              _)
                            (:OnInterrupted
                              _))
                          (Ability|EndAbility))))))
                (:OnInterrupted
                  (Ability|EndAbility))))))))))